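; BP_Ghost is a ghost Blueprint that switches its look between a normal and a power-up state.
; On BeginPlay it creates two dynamic material instances from the Sphere's material, recolors the power-up one pale tan, and clears the PowerUp flag.
; The ChangetoNormal and ChangetoPowerUp events swap the Sphere's material and update that flag, with no callers in this graph.
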(event EventBeginPlay
  (bind _sphere (Variables|Default|GetSphere))
  (bind _returnvalue (Rendering|Material|GetMaterial _sphere 0))
  (bind _returnvalue_2 (Rendering|Material|CreateDynamicMaterialInstance _returnvalue "None" :!class /Script/Engine.KismetMaterialLibrary))
  (Variables|Default|SetOriginal_Material _returnvalue_2)
  (bind _returnvalue_3 (Rendering|Material|CreateDynamicMaterialInstance _returnvalue "None" :!class /Script/Engine.KismetMaterialLibrary))
  (bind _output_get (Variables|Default|SetPowerUp_Material _returnvalue_3))
  (Rendering|Material|SetVectorParameterValue _output_get "Color" "(R=0.953125,G=0.831249,B=0.572983,A=1.000000)" :!class /Script/Engine.MaterialInstanceDynamic)
  (Variables|Default|Setpower_Up false))

(event EventChangetoNormal
  (Rendering|Material|SetMaterial (Variables|Default|GetSphere) 0 (Variables|Default|GetOriginal_Material))
  (Variables|Default|Setpower_Up false))

(event EventChangetoPowerUp
  (Rendering|Material|SetMaterial (Variables|Default|GetSphere) 0 (Variables|Default|GetPowerUp_Material))
  (Variables|Default|Setpower_Up true))

(fn ConstructionScript)